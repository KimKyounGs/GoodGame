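; BP_MainCharacter is the player character Blueprint, handling health, sniper scope UI and interaction with nearby actors.
; Damage clamps health and updates the health bar through BP_MainPlayerController, while a lazily created scope widget plays zoom animation and sound forward or reversed.
; An overlap radius tracks one BPI_Interactable target and toggles its state.
; Interact messages that target and switches to UI-only input with a cursor until CoversationClosed restores game input.
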(event `self.ShowSniperScopeWidget`
  (params (bShowScope :type Boolean))
  (bind _sniperscopewidget (`self.SniperScopeWidget`))
  (bind _sniperscopewidget_2 (`self.SniperScopeWidget`))
  ;[1 1 1] 스나이퍼 줌인
  (`/Engine/EditorBlueprintResources/StandardMacros.IsValid` (`self.SniperScopeWidget`)
    (:`Is Valid`
      _)
    (:`Is Not Valid`
      (bind _returnvalue (`|CreateWidget` "/Game/2Blueprints/HUD/WBP_SniperScope.WBP_SniperScope_C"))
      (bind _output_get (set `self.SniperScopeWidget` _returnvalue))
      (`UserWidget.AddToViewport` _output_get 0)))
  (if bShowScope
    (`/Engine/EditorBlueprintResources/StandardMacros.IsValid` _sniperscopewidget_2
      (:`Is Valid`
        (`UserWidget.PlayAnimation` _sniperscopewidget_2 (`/Game/2Blueprints/HUD/WBP_SniperScope.ScopeZoomIn` _sniperscopewidget_2) 0.0 1 "Forward" 1.0 false)
        (`GameplayStatics.PlaySound2D` "/Game/1Asset/MilitaryWeapSilver/Sound/SniperRifle/Wavs/SniperRifle_ZoomIn.SniperRifle_ZoomIn" 1.0 1.0 0.0 null null)))
    (else
      (`/Engine/EditorBlueprintResources/StandardMacros.IsValid` _sniperscopewidget
        (:`Is Valid`
          (`UserWidget.PlayAnimation` _sniperscopewidget (`/Game/2Blueprints/HUD/WBP_SniperScope.ScopeZoomIn` _sniperscopewidget) 0.0 1 "Reverse" 1.0 false)
          (`GameplayStatics.PlaySound2D` "/Game/1Asset/MilitaryWeapSilver/Sound/SniperRifle/Wavs/SniperRifle_ZoomOut.SniperRifle_ZoomOut" 1.0 1.0 0.0 null null))))))

(event `self.ReceiveBeginPlay`
  (set `self.CurrentHealth` (`self.Max_Health`))
  (bind _asbp_main_player_controller (cast `/Game/2Blueprints/PlayerController/BP_MainPlayerController` (`self.GetController`)))
  (`/Game/2Blueprints/PlayerController/BP_MainPlayerController.UpdateHealthbar` _asbp_main_player_controller (`self.CurrentHealth`) (`self.Max_Health`)))

(event `self.ReceiveTick`
  (params (DeltaSeconds :type "Float (single-precision)")))

(event `self.ReceiveAnyDamage`
  (params (Damage :type "Float (single-precision)") (DamageType :type "DamageType Object Reference") (InstigatedBy :type "Controller Object Reference") (DamageCauser :type "Actor Object Reference"))
  (set `self.CurrentHealth` (`KismetMathLibrary.FClamp` (- (`self.CurrentHealth`) Damage) 0.0 (`self.Max_Health`)))
  (bind _asbp_main_player_controller (cast `/Game/2Blueprints/PlayerController/BP_MainPlayerController` (`self.GetController`)))
  (`/Game/2Blueprints/PlayerController/BP_MainPlayerController.UpdateHealthbar` _asbp_main_player_controller (`self.CurrentHealth`) (`self.Max_Health`)))

(event `InputAction|Interact`
  (params (Key :type "Key Structure"))
  (:`Pressed`
    (`/Engine/EditorBlueprintResources/StandardMacros.IsValid` (`self.Interactable`)
      (:`Is Valid`
        (message `/Game/UI/Text_Script/BPI_Interactable.Interact` (`self.Interactable`) self)
        (`WidgetBlueprintLibrary.SetInputMode_UIOnlyEx` (`GameplayStatics.GetPlayerController` 0) null)
        (set `PlayerController.bShowMouseCursor` true (`GameplayStatics.GetPlayerController` 0))))))

(event `self.Interact_Radius.OnComponentBeginOverlap`
  (params (OverlappedComponent :type "PrimitiveComponent Object Reference") (OtherActor :type "Actor Object Reference") (OtherComp :type "PrimitiveComponent Object Reference") (OtherBodyIndex :type Integer) (bFromSweep :type Boolean) (SweepResult :type "HitResult Structure (by ref)"))
  (if (!= OtherActor self)
    (if (`KismetSystemLibrary.DoesImplementInterface` OtherActor "/Game/UI/Text_Script/BPI_Interactable.BPI_Interactable_C")
      (`/Engine/EditorBlueprintResources/StandardMacros.IsValid` (`self.Interactable`)
        (:`Is Valid`
          (message `/Game/UI/Text_Script/BPI_Interactable.Set_Interactable_State` (`self.Interactable`) false)
          (set `self.Interactable` null))
        (:`Is Not Valid`
          _))
      (set `self.Interactable` OtherActor)
      (message `/Game/UI/Text_Script/BPI_Interactable.Set_Interactable_State` (`self.Interactable`) true))))

(event `self.Interact_Radius.OnComponentEndOverlap`
  (params (OverlappedComponent :type "PrimitiveComponent Object Reference") (OtherActor :type "Actor Object Reference") (OtherComp :type "PrimitiveComponent Object Reference") (OtherBodyIndex :type Integer))
  (if (and (!= OtherActor self) (== (`self.Interactable`) OtherActor))
    (message `/Game/UI/Text_Script/BPI_Interactable.Set_Interactable_State` (`self.Interactable`) false)
    (set `self.Interactable` null)))

(event `/Game/UI/Text_Script/BPI_Interactable.Coversation_Closed`
  (set `PlayerController.bShowMouseCursor` false (`GameplayStatics.GetPlayerController` 0))
  (`WidgetBlueprintLibrary.SetInputMode_GameOnly` (`GameplayStatics.GetPlayerController` 0)))

(fn `UserConstructionScript`)